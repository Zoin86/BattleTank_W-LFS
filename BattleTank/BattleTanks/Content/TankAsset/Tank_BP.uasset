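; Player-drivable tank pawn that wires input and components together for movement, aiming, firing and a floating health bar.
; On BeginPlay it hands the tracks to TankMovement and the barrel and turret to TankAiming, then gives the health bar widget a reference to itself.
; Aim axes rotate an azimuth gimbal and spring arm for the camera, while drive axes and Fire forward to the movement and aiming components.
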(event EventBeginPlay
  (Class|TankMovementComponent|Initialise (Variables|Default|GetTankMovement) (Variables|Default|GetLeftTrack) (Variables|Default|GetRightTrack))
  (Class|TankAimingComponent|Initialise (Variables|Default|GetTankAiming) (Variables|Default|GetTankBarrel) (Variables|Default|GetTurret))
  (CallFunction|InitialiseHealthBarWidget))

(event Input|ActionEvents|InputActionFire
  (params (Key :type Key%20Structure))
  ;[1 1 1] Ballistics Binding
  (:Pressed
    (Class|TankAimingComponent|Fire (Variables|Default|GetTankAiming))))

(event Input|AxisEvents|InputAxisAimAzimuth
  (params (AxisValue :type Float%20%28single-precision%29))
  ;[1 1 1] Ballistics Binding
  (Transformation|AddLocalRotation (Variables|Default|GetAzimuth%20Gimbal%20%28Scene%20Component%29) (Math|Rotator|MakeRotator 0.0 0.0 AxisValue) false false))

(event Input|AxisEvents|InputAxisMoveForward
  (params (AxisValue :type Float%20%28single-precision%29))
  ;[1 1 1] Movement Input Binding
  (Class|TankMovementComponent|IntendMoveForward (Variables|Default|GetTankMovement) AxisValue))

(event Input|AxisEvents|InputAxisTurnRight
  (params (AxisValue :type Float%20%28single-precision%29))
  ;[1 1 1] Movement Input Binding
  (Class|TankMovementComponent|IntendTurnRight (Variables|Default|GetTankMovement) AxisValue))

(event Input|AxisEvents|InputAxisAimElevation
  (params (AxisValue :type Float%20%28single-precision%29))
  ;[1 1 1] Ballistics Binding
  (Transformation|AddLocalRotation (Variables|Default|GetSpringArm) (Math|Rotator|MakeRotator 0.0 AxisValue 0.0) false false))

(fn ConstructionScript)

(fn InitialiseHealthBarWidget
  (Variables|/Game/UI/FloatingHealthBarUI.FloatingHealthBarUI_C|SetMyTank_Ref (.AsFloating%20Health%20Bar%20UI (Utilities|Casting|CastToFloatingHealthBarUI (UserInterface|GetUserWidgetObject (Variables|Default|GetWidgetHealthBar)))) self))