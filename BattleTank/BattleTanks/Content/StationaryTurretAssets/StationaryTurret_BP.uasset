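; Stationary turret Blueprint that serves as an AI or placed gun emplacement with a floating health bar.
; On BeginPlay it initialises its TankAiming component with its barrel and turret parts.
; It then passes itself to the FloatingHealthBarUI widget on its widget component as the tank reference, so the bar can track this turret.
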(event EventBeginPlay
  (Class|TankAimingComponent|Initialise (Variables|Default|GetTankAiming) (Variables|Default|GetTankBarrel) (Variables|Default|GetTankTurret))
  (CallFunction|InitialiseWidget))

(fn ConstructionScript)

(fn InitialiseWidget
  (Variables|/Game/UI/FloatingHealthBarUI.FloatingHealthBarUI_C|SetMyTank_Ref (.AsFloating%20Health%20Bar%20UI (Utilities|Casting|CastToFloatingHealthBarUI (UserInterface|GetUserWidgetObject (Variables|Default|GetWidget)))) self))